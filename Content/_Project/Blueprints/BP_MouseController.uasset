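; BP_MouseController is a player controller that drives a viewport-style camera with mouse and keyboard through Enhanced Input.
; On BeginPlay it adds IMC_Viewport, shows the cursor and caches its BP_CameraManager, which receives look, move and scroll input.
; Chorded wheel input adjusts a clamped move speed, while unchorded wheel scrolls the camera.
; Right click hides the cursor while held; left click only prints debug text, and CameraZoom is an empty stub.
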(event `EnhancedInput|/Game/_Project/Input/Actions/Viewport/IA_RMB`
  (params (ActionValue :type Boolean) (ElapsedSeconds :type "Float (double-precision)") (TriggeredSeconds :type "Float (double-precision)") (InputAction :type "InputAction Object Reference" :default "/Game/_Project/Input/Actions/Viewport/IA_RMB.IA_RMB"))
  ;[1 1 1] Right click
  (:`Triggered`
    (set `self.bShowMouseCursor` false))
  (:`Canceled`
    (set `self.bShowMouseCursor` true :!label _label))
  (:`Completed`
    (goto _label)))

(event `EnhancedInput|/Game/_Project/Input/Actions/Viewport/IA_MouseMove`
  (params (ActionValue :type "Vector2D Structure") (ElapsedSeconds :type "Float (double-precision)") (TriggeredSeconds :type "Float (double-precision)") (InputAction :type "InputAction Object Reference" :default "/Game/_Project/Input/Actions/Viewport/IA_MouseMove.IA_MouseMove"))
  ;[1 1 1] Mouse Moe
  (:`Triggered`
    (`/Game/_Project/Blueprints/BP_CameraManager.CameraOrient` (`self.CameraManager`) ActionValue 1.0)))

(event `EnhancedInput|/Game/_Project/Input/Actions/Viewport/IA_MouseWheelChorded`
  (params (ActionValue :type "Float (double-precision)") (ElapsedSeconds :type "Float (double-precision)") (TriggeredSeconds :type "Float (double-precision)") (InputAction :type "InputAction Object Reference" :default "/Game/_Project/Input/Actions/Viewport/IA_MouseWheelChorded.IA_MouseWheelChorded"))
  (:`Triggered`
    (`self.ModifyCameraMoveSpeed` ActionValue)))

(event `EnhancedInput|/Game/_Project/Input/Actions/Viewport/IA_WASD`
  (params (ActionValue :type "Vector2D Structure") (ElapsedSeconds :type "Float (double-precision)") (TriggeredSeconds :type "Float (double-precision)") (InputAction :type "InputAction Object Reference" :default "/Game/_Project/Input/Actions/Viewport/IA_WASD.IA_WASD"))
  (:`Triggered`
    (`/Game/_Project/Blueprints/BP_CameraManager.CameraMove` (`self.CameraManager`) ActionValue (`self.CameraMoveSpeed`))))

(event `EnhancedInput|/Game/_Project/Input/Actions/Viewport/IA_MouseWheelUnchorded`
  (params (ActionValue :type "Float (double-precision)") (ElapsedSeconds :type "Float (double-precision)") (TriggeredSeconds :type "Float (double-precision)") (InputAction :type "InputAction Object Reference" :default "/Game/_Project/Input/Actions/Viewport/IA_MouseWheelUnchorded.IA_MouseWheelUnchorded"))
  (:`Triggered`
    (`/Game/_Project/Blueprints/BP_CameraManager.ScrollMouse` (`self.CameraManager`) ActionValue (`self.CameraScrollSpeed`))))

(event `EnhancedInput|/Game/_Project/Input/Actions/Viewport/IA_LMB`
  (params (ActionValue :type Boolean) (ElapsedSeconds :type "Float (double-precision)") (TriggeredSeconds :type "Float (double-precision)") (InputAction :type "InputAction Object Reference" :default "/Game/_Project/Input/Actions/Viewport/IA_LMB.IA_LMB"))
  (:`Triggered`
    (`KismetSystemLibrary.PrintString` "LMB")))

(event `self.ReceiveBeginPlay`
  (`WidgetBlueprintLibrary.SetInputMode_GameAndUIEx` self null "LockOnCapture")
  (set `self.bShowMouseCursor` true)
  (`self.EnableEnhancedInput`)
  (`self.CacheCameraManager`))

(fn `CacheCameraManager`
  (bind _asbp_camera_manager (cast `/Game/_Project/Blueprints/BP_CameraManager` (`self.PlayerCameraManager`)))
  (set `self.CameraManager` _asbp_camera_manager))

(fn `CameraZoom`
  (params (InputValue :type "Float (double-precision)")))

(fn `EnableEnhancedInput`
  (`EnhancedInputSubsystemInterface.AddMappingContext` (subsystem `EnhancedInputLocalPlayerSubsystem`) "/Game/_Project/Input/IMC_Viewport.IMC_Viewport" 0 (struct)))

(fn `ModifyCameraMoveSpeed`
  (params (Input :type "Float (double-precision)"))
  (set `self.CameraMoveSpeed` (`KismetMathLibrary.FClamp` (+ (`self.CameraMoveSpeed`) (* Input 1.0)) 1.0 100.0)))

(fn `UserConstructionScript`)