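; Player camera manager that drives a free-moving camera, starting at an offset from the controlled pawn and looking straight down.
; It stores its own location and rotation, which BlueprintUpdateCamera returns each update with the default FOV, ignoring the view target.
; ScrollMouse and CameraMove translate along the camera's forward and right vectors, while CameraOrient adds input to pitch and yaw without applying its Scale.
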(event `self.ReceiveBeginPlay`
  (`self.SetStartingLocation`)
  (`self.SetStartingRotation`))

(fn `BlueprintUpdateCamera`
  (params (CameraTarget :type "Actor Object Reference"))
  (returns (NewCameraLocation :type "Vector Structure") (NewCameraRotation :type "Rotator Structure") (NewCameraFOV :type "Float (single-precision)") (ReturnValue :type Boolean))
  (return (`self.CurrentCameraLocation`) (`self.CurrentCameraRotation`) (`self.DefaultFOV`) true))

(fn `CameraMove`
  (params (InputValue :type "Vector2D Structure") (Scale :type "Float (double-precision)"))
  (bind (_x _y) (`KismetMathLibrary.BreakVector2D` InputValue))
  (bind _currentcamerarotation (`self.CurrentCameraRotation`))
  (set `self.CurrentCameraLocation` (+ (* _x Scale (`KismetMathLibrary.GetForwardVector` _currentcamerarotation)) (`self.CurrentCameraLocation`) (* _y Scale (`KismetMathLibrary.GetRightVector` _currentcamerarotation)))))

(fn `CameraOrient`
  (params (InputValue :type "Vector2D Structure") (Scale :type "Float (double-precision)"))
  (bind (_currentcamerarotation_roll _currentcamerarotation_pitch _currentcamerarotation_yaw) (`KismetMathLibrary.BreakRotator` (`self.CurrentCameraRotation`)))
  (set `self.CurrentCameraRotation` (`KismetMathLibrary.MakeRotator` _currentcamerarotation_roll (+ InputValue_Y _currentcamerarotation_pitch) (+ _currentcamerarotation_yaw InputValue_X))))

(fn `ScrollMouse`
  (params (InputValue :type "Float (double-precision)") (Scale :type "Float (double-precision)"))
  (set `self.CurrentCameraLocation` (+ (* InputValue Scale (`KismetMathLibrary.GetForwardVector` (`self.CurrentCameraRotation`))) (`self.CurrentCameraLocation`))))

(fn `SetStartingLocation`
  (bind _asplayer_controller (cast `PlayerController` (`self.GetOwner`)))
  (set `self.CurrentCameraLocation` (+ (`self.K2_GetActorLocation` (`Controller.K2_GetPawn` _asplayer_controller)) (`self.StartingOffset`))))

(fn `SetStartingRotation`
  (set `self.CurrentCameraRotation` (`KismetMathLibrary.Conv_VectorToRotator` (`KismetMathLibrary.Vector_Down`))))

(fn `UserConstructionScript`)