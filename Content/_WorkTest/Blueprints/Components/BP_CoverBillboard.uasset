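; BP_CoverBillboard is a component that draws debug gizmos, apparently to visualize a cover point on its owning actor.
; DrawGizmos draws a long-lived circle at the component, aligned to the owner's forward and right axes.
; It also traces on Visibility toward the owner's location and draws a short arrow along the hit normal, flattened horizontally.
; BeginPlay and Tick are unused.
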(event `self.DrawGizmos`
  (bind _returnvalue (`self.K2_GetComponentLocation`))
  (bind _returnvalue_2 (`self.K2_GetComponentLocation`))
  (bind _returnvalue_3 (`self.GetOwner`))
  (`KismetSystemLibrary.DrawDebugCircle` _returnvalue_2 50.0 10 (struct :`R` 0.185232 :`G` 1.0 :`A` 1.0) 999999.0 5.0 (`Actor.GetActorRightVector` _returnvalue_3) (`Actor.GetActorForwardVector` _returnvalue_3))
  (bind _outhit (`KismetSystemLibrary.LineTraceSingle` :`Start` _returnvalue_2 :`End` (`Actor.K2_GetActorLocation` _returnvalue_3) :`TraceChannel` "TraceTypeQuery1" :`DrawDebugType` "ForDuration" :`bIgnoreSelf` false))
  (`KismetSystemLibrary.DrawDebugArrow` _returnvalue (+ _returnvalue (* (`KismetMathLibrary.ProjectVectorOnToPlane` (`.Normal` (`GameplayStatics.BreakHitResult` _outhit)) (`KismetMathLibrary.Vector_Up`)) 10)) 2.0 (struct :`G` 0.100078 :`B` 1.0 :`A` 1.0) 5.0 2.0))